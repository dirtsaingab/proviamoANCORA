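; Player character for a side-on platformer: moves along X, jumps with buffering and coyote time, attacks, and interacts via BP_Interact.
; Tick flips control rotation by velocity and traces below the feet while falling, toggling capsule collision to land on platforms.
; Falling onto enemies defeats them and bounces; other enemy contact defeats the player, triggering feedback and a delayed GameMode restart.
; Attack animation blocks new input; hit box overlaps only print enemy names.
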(event `self.ReceiveBeginPlay`
  (`parent.ReceiveBeginPlay`)
  (bind _asplayer_controller (cast `PlayerController` (`self.GetController`)))
  (`EnhancedInputSubsystemInterface.AddMappingContext` (pcsubsystem `EnhancedInputLocalPlayerSubsystem` _asplayer_controller) "/Game/Input/IMC_Platformer.IMC_Platformer" 0 (struct))
  (`self.SetHitBoxCollusion` false)
  (add `self.Defeated` (delegate `OnDefeated`)))

(event `OnDefeated`
  (bind _asgm_platformer (cast `/Game/Blieprints/GM_Platformer` (`GameplayStatics.GetGameMode`)))
  (`KismetSystemLibrary.Delay` 2.0)
  (`/Game/Blieprints/GM_Platformer.RestartGame` _asgm_platformer))

(event `self.ReceiveTick`
  (params (DeltaSeconds :type "Float (single-precision)"))
  (`parent.ReceiveTick` DeltaSeconds)
  (`self.UdateControlRotation`)
  (`self.TraceForPlatform`)
  (if (and (`self.IsJumpBuffering`) (`self.CanJump`))
    (`self.Jump`)))

(event `EnhancedInput|/Game/Input/Action/IA_Jump`
  (params (ActionValue :type Boolean) (ElapsedSeconds :type "Float (double-precision)") (TriggeredSeconds :type "Float (double-precision)") (InputAction :type "InputAction Object Reference" :default "/Game/Input/Action/IA_Jump.IA_Jump"))
  (:`Started`
    (if (not (`self.IsAttacking`))
      (if (`self.CanJump`)
        (`self.Jump`)
        (else
          (set `self.IsJumpBuffering` true)
          (`KismetSystemLibrary.RetriggerableDelay` (`self.JumpBufferLenght`))
          (set `self.IsJumpBuffering` false)))))
  (:`Completed`
    (`self.StopJumping`)))

(event `self.OnWalkingOffLedge`
  (params (PreviousFloorImpactNormal :type "Vector Structure (by ref)") (PreviousFloorContactNormal :type "Vector Structure (by ref)") (PreviousLocation :type "Vector Structure (by ref)") (TimeDelta :type "Float (single-precision)"))
  (set `self.IsInCayoteTime` true)
  (`KismetSystemLibrary.RetriggerableDelay` (`self.CoyateTimeLenght`))
  (set `self.IsInCayoteTime` false))

(event `EnhancedInput|/Game/Input/Action/IA_Move`
  (params (ActionValue :type "Float (double-precision)") (ElapsedSeconds :type "Float (double-precision)") (TriggeredSeconds :type "Float (double-precision)") (InputAction :type "InputAction Object Reference" :default "/Game/Input/Action/IA_Move.IA_Move"))
  (:`Triggered`
    (if (not (`self.IsAttacking`))
      (`self.AddMovementInput` (1.0 0.0 0.0) ActionValue))))

(event `self.CapsuleComponent.OnComponentBeginOverlap`
  (params (OverlappedComponent :type "PrimitiveComponent Object Reference") (OtherActor :type "Actor Object Reference") (OtherComp :type "PrimitiveComponent Object Reference") (OtherBodyIndex :type Integer) (bFromSweep :type Boolean) (SweepResult :type "HitResult Structure (by ref)"))
  (bind (_returnvalue_x _returnvalue_y _returnvalue_z) (`KismetMathLibrary.BreakVector` (`self.GetVelocity`)))
  (bind _asbp_enemy (cast `/Game/Blieprints/Characters/Enemy/BP_Enemy` OtherActor))
  (if (and (`NavMovementComponent.IsFalling` (`self.CharacterMovement`)) (< _returnvalue_z 0.0))
    (`self.Defeat` _asbp_enemy)
    (`self.LaunchCharacter` (`KismetMathLibrary.MakeVector` 0.0 0.0 (`self.EnemyBounceLounge`)) false true)
    (else
      (`self.Defeat`))))

(event `self.Defeat`
  (`parent.Defeat`)
  (bind _asplayer_controller (cast `PlayerController` (`self.GetController`)))
  (`EnhancedInputSubsystemInterface.RemoveMappingContext` (pcsubsystem `EnhancedInputLocalPlayerSubsystem` _asplayer_controller) "/Game/Input/IMC_Platformer.IMC_Platformer" (struct))
  (`SceneComponent.K2_DetachFromComponent` (`self.SpringArm`) "KeepWorld" "KeepRelative" "KeepRelative" true)
  (`GameplayStatics.PlaySound2D` "/Game/Assets/Sound/PlayerDefeated/S_PlayerDefeated_Cue.S_PlayerDefeated_Cue" 1.0 1.0 0.0 null null)
  (`GameplayStatics.PlayWorldCameraShake` "/Game/CameraShake/CS_Defeated.CS_Defeated_C" (`self.K2_GetActorLocation`) 0.0 10000.0 0.0))

(event `EnhancedInput|/Game/Input/Action/IA_Attack`
  (params (ActionValue :type Boolean) (ElapsedSeconds :type "Float (double-precision)") (TriggeredSeconds :type "Float (double-precision)") (InputAction :type "InputAction Object Reference" :default "/Game/Input/Action/IA_Attack.IA_Attack"))
  (:`Started`
    (if (not (`self.IsAttacking`))
      (`PaperZDPlaySlotOverrideAction.PlayAnimationOverrideWithCallbacks` (`self.GetAnimInstance`) "/Game/Blieprints/Characters/Player/AnimSequences/Attack.Attack"
        (:`then`
          (set `self.IsAttacking` true))
        (:`OnCompleted`
          (set `self.IsAttacking` false :!label _label))
        (:`OnCancelled`
          (goto _label))))))

(event `self.Box.OnComponentBeginOverlap`
  (params (OverlappedComponent :type "PrimitiveComponent Object Reference") (OtherActor :type "Actor Object Reference") (OtherComp :type "PrimitiveComponent Object Reference") (OtherBodyIndex :type Integer) (bFromSweep :type Boolean) (SweepResult :type "HitResult Structure (by ref)"))
  (bind _asbp_enemy (cast `/Game/Blieprints/Characters/Enemy/BP_Enemy` OtherActor))
  (`KismetSystemLibrary.PrintString` (`KismetSystemLibrary.GetDisplayName` _asbp_enemy)))

(event `Key|E`
  (params (Key :type "Key Structure"))
  (:`Pressed`
    (for _array_element (`self.GetOverlappingActors` "/Script/Engine.Actor")
      (if (`KismetSystemLibrary.DoesImplementInterface` _array_element "/Game/Blieprints/BP_Interact.BP_Interact_C")
        (message `/Game/Blieprints/BP_Interact.Interact` _array_element)
        (break)))))

(fn `CanJumpInternal`
  (returns (ReturnValue :type Boolean))
  (bind _returnvalue (`parent.CanJumpInternal`))
  (return (or _returnvalue (`self.IsInCayoteTime`))))

(fn `SetHitBoxCollusion`
  (params (SetActive :type Boolean))
  (if SetActive
    (`PrimitiveComponent.SetCollisionEnabled` (`self.Box`) "QueryOnly")
    (else
      (`PrimitiveComponent.SetCollisionEnabled` (`self.Box`) "NoCollision"))))

(fn `TraceForPlatform`
  (bind (_returnvalue_x _returnvalue_y _returnvalue_z) (`KismetMathLibrary.BreakVector` (`self.GetVelocity`)))
  (bind _returnvalue (`SceneComponent.K2_GetComponentLocation` (`self.FootPosition`)))
  (if (`NavMovementComponent.IsFalling` (`self.CharacterMovement`))
    (bind (_outhit _returnvalue_2) (`KismetSystemLibrary.LineTraceSingleForObjects` _returnvalue (+ _returnvalue (* (`KismetMathLibrary.Vector_Down`) (`self.PlatformCheckDistance`))) (`|MakeArray` "ObjectTypeQuery7" :!type "EObjectTypeQuery Enum")))
    (if (and _returnvalue_2 (< _returnvalue_z 0.0))
      (`PrimitiveComponent.SetCollisionResponseToChannel` (`self.CapsuleComponent`) "ECC_GameTraceChannel1" "ECR_Block")
      (else
        (`PrimitiveComponent.SetCollisionResponseToChannel` (`self.CapsuleComponent`) "ECC_GameTraceChannel1" "ECR_Overlap")))))

(fn `UdateControlRotation`
  (bind _returnvalue (`self.GetController`))
  (bind _returnvalue_2 (`self.GetController`))
  (bind _velocity_x (`KismetMathLibrary.BreakVector` (`MovementComponent.Velocity` (`self.CharacterMovement`))))
  (`/Engine/EditorBlueprintResources/StandardMacros.CompareFloat` _velocity_x
    (:`>`
      (`/Engine/EditorBlueprintResources/StandardMacros.IsValid` _returnvalue_2
        (:`Is Valid`
          (`Controller.SetControlRotation` _returnvalue_2 (`KismetMathLibrary.MakeRotator` 0.0)))))
    (:`<`
      (`/Engine/EditorBlueprintResources/StandardMacros.IsValid` _returnvalue
        (:`Is Valid`
          (`Controller.SetControlRotation` _returnvalue (`KismetMathLibrary.MakeRotator` 0.0 0.0 180.0)))))))

(fn `UserConstructionScript`
  (`parent.UserConstructionScript`))